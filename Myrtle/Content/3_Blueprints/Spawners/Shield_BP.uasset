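; Shield pickup actor that gives the player character a shield when touched.
; On sphere overlap with BP_ThirdPersonCharacter, it sets that character's shield amount to its SheildHP, snaps itself onto the character and flags itself as picked up.
; Once picked up, it polls the shield amount of player 0's character every tick and destroys itself when the value drops below zero.
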(event OnComponentBeginOverlap(Sphere1)
  (params (OverlappedComponent :type Primitive%20Component%20Object%20Reference) (OtherActor :type Actor%20Object%20Reference) (OtherComp :type Primitive%20Component%20Object%20Reference) (OtherBodyIndex :type Integer) (bFromSweep :type Boolean) (SweepResult :type Hit%20Result%20Structure%20%28by%20ref%29))
  (bind _asbp_third_person_character (Utilities|Casting|CastToBP_ThirdPersonCharacter OtherActor))
  (Variables|/Game/ThirdPerson/Blueprints/BP_ThirdPersonCharacter.BP_ThirdPersonCharacter_C|SetPlayerSheildAmount _asbp_third_person_character (Variables|Default|GetSheildHP))
  (Transformation|AttachActorToActor _asbp_third_person_character "None" "SnapToTarget" "SnapToTarget" "SnapToTarget" true)
  (Variables|Default|SetPicked%20Up? true))

(event EventTick
  (params (DeltaSeconds :type Float%20%28single-precision%29))
  (if (Variables|Default|GetPicked%20Up?)
    (bind _asbp_third_person_character (Utilities|Casting|CastToBP_ThirdPersonCharacter (Game|GetPlayerCharacter 0)))
    (if (< (Variables|/Game/ThirdPerson/Blueprints/BP_ThirdPersonCharacter.BP_ThirdPersonCharacter_C|GetPlayerSheildAmount _asbp_third_person_character) 0.0)
      (Actor|DestroyActor))))

(fn ConstructionScript)