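; Enemy AI character that chases the first player character and shows its health on a widget.
; After a one-second delay it destroys itself if falling, otherwise starts an AIMoveTo loop that retries half a second after success or failure.
; A capsule hit with BP_ThirdPersonCharacter sets the enemy's own Health to zero.
; UpdateHealthBar copies Health into the Enemey_Stats_Widget, though nothing in these graphs calls it.
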(event OnComponentHit(CapsuleComponent)
  (params (HitComponent :type Primitive%20Component%20Object%20Reference) (OtherActor :type Actor%20Object%20Reference) (OtherComp :type Primitive%20Component%20Object%20Reference) (NormalImpulse :type Vector :default "0, 0, 0") (Hit :type Hit%20Result%20Structure%20%28by%20ref%29))
  (Utilities|Casting|CastToBP_ThirdPersonCharacter OtherActor)
  (Variables|Default|SetHealth 0.0))

(event Custom|Ai%20Move%20To
  (AI|AIMoveTo (Class|PawnMovementComponent|GetPawnOwner (Variables|Character|GetCharacterMovement)) "0, 0, 0" (Game|GetPlayerCharacter 0) 1.0 false
    (:OnSuccess
      _)
    (:OnFail
      _))
  (Utilities|FlowControl|Delay 0.5)
  (CallFunction|AiMoveto))

(event EventBeginPlay
  (Utilities|FlowControl|Delay 1.0)
  (if (AI|Components|NavMovement|IsFalling (Variables|Character|GetCharacterMovement))
    (Actor|DestroyActor)
    (else
      (CallFunction|AiMoveto))))

(fn ConstructionScript)

(fn UpdateHealthBar
  (bind _asenemey_stats_widget (Utilities|Casting|CastToEnemey_Stats_Widget (UserInterface|GetUserWidgetObject (Variables|Default|GetHealthWidget))))
  (Variables|/Game/3_Blueprints/Enemies/Enemey_001/Enemey_Stats_Widget.Enemey_Stats_Widget_C|SetAI_Widget_Health _asenemey_stats_widget (Variables|Default|GetHealth)))